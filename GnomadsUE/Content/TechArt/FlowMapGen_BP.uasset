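; Prototype flow map generator that tracks a trail of particles left by the moving player, in player-centred 0–1 space.
; Tick spawns particles at the centre on movement, shifts them against player motion scaled by MaxDistToPlayer, and periodically drops the oldest.
; Positions are packed as one-pixel colours into the LocArray render target and copied to a texture via an editor-only conversion.
; Tick also draws a material into RT2.
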(event Custom|CreateParticleInformation
  (bind _locarray (Variables|Default|GetLocArray))
  (bind (_canvas _size _context) (Rendering|BeginDrawCanvastoRenderTarget _locarray))
  (Variables|Default|SetCanvas _canvas)
  (Variables|Default|SetContext _context)
  (for (_array_element _array_index) (Variables|Default|GetParticleLocations)
    (Canvas|DrawTexture :self (Variables|Default|GetCanvas) :ScreenPosition (Math|Vector2D|MakeVector2D (Math|Conversions|ToFloat(Integer) _array_index) 0.0) :ScreenSize "(X=1.000000,Y=1.000000)" :CoordinateSize "(X=1.000000,Y=1.000000)" :RenderColor (Math|Conversions|ToLinearColor(Vector) _array_element) :BlendMode "BLEND_Opaque" :PivotPoint "(X=0.500000,Y=0.500000)"))
  (Rendering|EndDrawCanvastoRenderTarget (Variables|Default|GetContext))
  (EditorScripting|Rendering|ConvertRenderTargettoTexture2DEditorOnly _locarray (Variables|Default|GetOutput)))

(event Custom|UpdateParticleInformation
  (bind _returnvalue (Game|GetPlayerCharacter 0))
  (bind _particlelocations (Variables|Default|GetParticleLocations))
  (bind _mesh (Variables|/Script/Engine.Character|GetMesh _returnvalue))
  (bind _returnvalue_2 (Transformation|GetWorldLocation _mesh))
  ;[1 1 1] Place new Particle
  (if (< (Variables|Default|GetDist) 0.01)
    ;[1 1 1] Get character Locations compared to particles (if particles to character is > 0; move particles;
    (Variables|Default|SetPlayerWorldLoc _returnvalue_2)
    (else
      (bind _output_get (Variables|Default|SetDir (Math|Vector|Normalize (- (Variables|Default|GetPlayerWorldLoc) _returnvalue_2))))
      (Variables|Default|SetPlayerWorldLoc _returnvalue_2)
      (for (_array_element _array_index) _particlelocations
        (Utilities|Array|SetArrayElem _particlelocations _array_index (+ _array_element (* (* (/ 1.0 (Variables|Default|GetMaxDistToPlayer)) (Variables|Default|GetDist)) _output_get))))))
  (CallFunction|CreateParticleInformation))

(event Custom|SpawnNewParticle
  (Utilities|Array|Add (Variables|Default|GetParticleLocations) "0.500000,0.500000,0.000000")
  (Utilities|Array|Add :TargetArray (Variables|Default|GetParticleDirAndLife)))

(event EventBeginPlay
  (Variables|Default|SetPlayerWorldLoc (Transformation|GetWorldLocation (Variables|/Script/Engine.Character|GetMesh (Game|GetPlayerCharacter 0))))
  (Rendering|ClearRenderTarget2D (Variables|Default|GetLocArray)))

(event EventTick
  (params (DeltaSeconds :type Float%20%28single-precision%29))
  (bind _result (Math|Integer|IncrementInt (Variables|Default|GetTEMPORARYTimer))
    (:%20%20
      (if (> _result 2)
        (Utilities|Array|RemoveIndex (Variables|Default|GetParticleLocations))
        (Rendering|DrawMaterialtoRenderTarget "/Game/TechArt/RT2.RT2" (Variables|Default|GetMaterial))
        (CallFunction|UpdateParticleInformation)
        (Variables|Default|SetTEMPORARYTimer 0)
        (else
          (bind _output_get (Variables|Default|SetDist (Math|Vector|Distance(Vector) (Variables|Default|GetPlayerWorldLoc) (Transformation|GetWorldLocation (Variables|/Script/Engine.Character|GetMesh (Game|GetPlayerCharacter 0))))))
          (if (> _output_get 0.0)
            ;[1 1 1] Spawn New Particle
            (CallFunction|SpawnNewParticle))
          (Rendering|DrawMaterialtoRenderTarget "/Game/TechArt/RT2.RT2" (Variables|Default|GetMaterial))
          (CallFunction|UpdateParticleInformation)
          (Variables|Default|SetPlayerWorldLoc (Transformation|GetWorldLocation (Variables|/Script/Engine.Character|GetMesh (Game|GetPlayerCharacter 0)))))))))