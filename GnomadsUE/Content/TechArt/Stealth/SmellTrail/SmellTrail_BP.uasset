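; Smell trail actor for stealth that records the player's path on a spline and checks whether the cat AI is near it.
; A looping timer appends the player's location, then removes the oldest point after a delay.
; A faster timer finds the cat by class and measures its distance to the closest spline location.
; Coming within range only prints a debug message, with no AI response here.
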(event Custom|HandleCatCollision
  (bind _returnvalue (Actor|GetActorOfClass "/Game/Characters/Cat/CatAI_BluePrint.CatAI_BluePrint_C"))
  (if (< (Math|Vector|Distance(Vector) (Spline|FindLocationClosesttoWorldLocation (Variables|Default|GetSpline) (Transformation|GetActorLocation _returnvalue) "World") (Transformation|GetActorLocation _returnvalue)) 5e+02)
    (Development|PrintString "Smells")))

(event Custom|EditSpline
  (Spline|AddSplinePoint (Variables|Default|GetSpline) (Transformation|GetActorLocation (Game|GetPlayerCharacter 0)) "World" true)
  (Utilities|FlowControl|Delay 0.6)
  (Spline|RemoveSplinePoint (Variables|Default|GetSpline) 0 true))

(event EventBeginPlay
  (bind _spline (Variables|Default|GetSpline))
  (Spline|AddSplinePoint _spline (Transformation|GetActorLocation (Game|GetPlayerCharacter 0)) "World" true)
  (Spline|RemoveSplinePoint _spline 0 true)
  (Utilities|Time|SetTimerbyEvent (delegate Custom|EditSpline) 0.5 true)
  (Utilities|Time|SetTimerbyEvent (delegate Custom|HandleCatCollision) 0.1 true))

(fn ConstructionScript)