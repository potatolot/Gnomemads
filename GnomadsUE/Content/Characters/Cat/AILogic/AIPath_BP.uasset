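; AI path actor, filed under the cat's AI logic, that manages an ordered array of AIMovePoint_BP waypoints.
; Events spawn numbered points at the path or a given transform, attach them with absolute location, and delete by index or last.
; AddTempPoint appends a point, then after a short delay deletes index zero, without renumbering.
; Getters return point count and location by index, printing debug strings.
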(event Custom|AddTempPoint
  (params (Transform :type Transform))
  (CallFunction|AddPointat Transform)
  (Utilities|FlowControl|Delay 1.0)
  (CallFunction|DeletePoint))

(event Custom|AddPointAt
  (params (Location :type Transform))
  (bind _returnvalue (Game|SpawnActorfromClass "/Game/Characters/Cat/AILogic/AIMovePoint_BP.AIMovePoint_BP_C" Location "Undefined" "MultiplyWithRoot" 0 0))
  (Transformation|SetAbsolute (Variables|/Game/Characters/Cat/AILogic/AIMovePoint_BP.AIMovePoint_BP_C|GetDefaultSceneRoot _returnvalue) true false false)
  (bind _returnvalue_2 (Utilities|Array|Add (Variables|Default|GetPoints) _returnvalue))
  (Default|SetNumber _returnvalue _returnvalue_2)
  (Transformation|AttachActorToActor _returnvalue self "None" "KeepRelative" "KeepRelative" "KeepRelative" true))

(event Custom|AddPoint
  ;[1 1 1] Add Point as Child
  (bind _returnvalue (Game|SpawnActorfromClass "/Game/Characters/Cat/AILogic/AIMovePoint_BP.AIMovePoint_BP_C" (Transformation|GetActorTransform) "Undefined" "MultiplyWithRoot" 0 0))
  (Transformation|SetAbsolute (Variables|/Game/Characters/Cat/AILogic/AIMovePoint_BP.AIMovePoint_BP_C|GetDefaultSceneRoot _returnvalue) true false false)
  (bind _returnvalue_2 (Utilities|Array|Add (Variables|Default|GetPoints) _returnvalue))
  (Default|SetNumber _returnvalue _returnvalue_2)
  (Transformation|AttachActorToActor _returnvalue self "None" "KeepRelative" "KeepRelative" "KeepRelative" true))

(event Custom|DeleteLast
  (CallFunction|DeletePoint (- (Utilities|Array|Length (Variables|Default|GetPoints)) 1)))

(event Custom|DeletePoint
  (params (Index :type Integer))
  (bind _points (Variables|Default|GetPoints))
  (Actor|DestroyActor (Utilities|Array|Get(acopy) _points Index))
  (Utilities|Array|RemoveIndex _points Index))

(event EventBeginPlay)

(event Collision|EventActorBeginOverlap
  (params (OtherActor :type Actor%20Object%20Reference)))

(event EventTick
  (params (DeltaSeconds :type Float%20%28single-precision%29)))

(fn ConstructionScript)

(fn GetLocationbyIndex
  (params (Index :type Integer))
  (Development|PrintString (Utilities|String|ToString(Integer) Index))
  (return (Transformation|GetActorLocation (Utilities|Array|Get(acopy) (Variables|Default|GetPoints) Index))))

(fn GetPathPointCount
  (bind _points (Variables|Default|GetPoints))
  (bind _returnvalue (Utilities|Array|Length _points))
  (Development|PrintString (Utilities|String|Append "The value is : " (Utilities|String|ToString(Integer) _returnvalue)))
  (return _returnvalue))