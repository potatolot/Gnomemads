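; Player audio component (a backup copy, by its name) that drives FMOD music, ambience and player sound effects.
; BeginPlay sets global parameters and starts forest, cave and ambience events, which EndPlay stops.
; Gameplay events map cat alert and grass hiding to global parameters, and play whistle, pickup and drop sounds, with a downward trace detecting water.
; Environment events only update EnvironmentType, which reaches FMOD only at BeginPlay.
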(event Custom|DropObject
  ;[0.3101 0.5806 0.6875] Pick up objects
  (Class|FMODBlueprintStatics|PlayEvent2D "/Game/FMOD/Events/Environment/Player/IdleCloth/Player_Idle_3.Player_Idle_3")
  (CallFunction|DropObjectonSurface))

(event Custom|Whistle
  (params (bIsDoubleWhistle :type Boolean))
  ;[0.3101 0.5806 0.6875] Whistle
  (if bIsDoubleWhistle
    (Class|FMODBlueprintStatics|PlayEvent2D "/Game/FMOD/Events/Environment/Player/PlayerActions/Player_WhistleDouble.Player_WhistleDouble")
    (else
      (Class|FMODBlueprintStatics|PlayEvent2D "/Game/FMOD/Events/Environment/Player/PlayerActions/Player_WhistleShort.Player_WhistleShort"))))

(event Custom|HiddenInGrass
  (params (State :type Boolean))
  ;[0.3101 0.6875 0.3314] Hidden in Grass
  (if State
    (Class|FMODBlueprintStatics|SetGlobalParameterbyName "HiddenInGrass" 1.0)
    (else
      (Class|FMODBlueprintStatics|SetGlobalParameterbyName "HiddenInGrass" 0.0))))

(event Custom|PickUpObject
  ;[0.3101 0.5806 0.6875] Pick up objects
  (Class|FMODBlueprintStatics|PlayEvent2D "/Game/FMOD/Events/Environment/Player/IdleCloth/Player_Idle_4.Player_Idle_4"))

(event Custom|CatTriggeredMusic
  (params (CatTriggeredTimer :type Float%20%28double-precision%29))
  ;[0.5938 0.1855 0.1855] Music behaviour for cat
  (bind _output_get (Variables|Cat|SetCatTriggeredTimer CatTriggeredTimer))
  (if (> _output_get 0.99)
    (Class|FMODBlueprintStatics|SetGlobalParameterbyName "PlayerNoise" 1.0)
    (else
      (Class|FMODBlueprintStatics|SetGlobalParameterbyName "RiserDanger" (Variables|Cat|GetCatTriggeredTimer))
      (if (< (Variables|Cat|GetCatTriggeredTimer) 0.01)
        (Class|FMODBlueprintStatics|SetGlobalParameterbyName "PlayerNoise" 0.0)))))

(event Custom|EnterForest
  ;[0.3101 0.6875 0.3314] Set Environment
  (Variables|Default|SetEnvironmentType 1.5))

(event Custom|EnterCave
  ;[0.3101 0.6875 0.3314] Set Environment
  (Variables|Default|SetEnvironmentType 3.0))

(event Custom|EnterHouse
  ;[0.3101 0.6875 0.3314] Set Environment
  (Variables|Default|SetEnvironmentType 0.0))

(event EventEndPlay
  (params (EndPlayReason :type EEndPlayReason%20Enum :default "Destroyed"))
  ;[0.5938 0.1855 0.1855] Music system Start/Stop
  (Class|FMODBlueprintStatics|EventInstanceStop (stale EventBeginPlay _returnvalue) false)
  (Class|FMODBlueprintStatics|EventInstanceStop (stale EventBeginPlay _returnvalue_2) false)
  (Class|FMODBlueprintStatics|EventInstanceStop (stale EventBeginPlay _returnvalue_3) false))

(event EventBeginPlay
  ;[0.375 0.375 0.375] Fmod Global Sliders Init
  (Utilities|FlowControl|Sequence
    (:then_0
      (Class|FMODBlueprintStatics|SetGlobalParameterbyName "PlayerNoise" (Variables|Default|GetNoiseLevel))
      (Class|FMODBlueprintStatics|SetGlobalParameterbyName "Environment" (Variables|Default|GetEnvironmentType))
      (Class|FMODBlueprintStatics|SetGlobalParameterbyName "RiserDanger" (Variables|Default|GetRiserDanger)))
    (:then_1
      ;[0.5938 0.1855 0.1855] Music system Start/Stop
      (bind _returnvalue (Class|FMODBlueprintStatics|PlayEvent2D "/Game/FMOD/Events/Music/Forest.Forest"))
      (bind _returnvalue_2 (Class|FMODBlueprintStatics|PlayEvent2D "/Game/FMOD/Events/Environment/Rough_ambience.Rough_ambience"))
      (bind _returnvalue_3 (Class|FMODBlueprintStatics|PlayEvent2D "/Game/FMOD/Events/Music/Cave.Cave")))))

(fn DropObjectonSurface
  (bind _returnvalue (Components|GetOwner))
  (bind _returnvalue_2 (Transformation|GetActorLocation _returnvalue))
  (bind _returnvalue_3 (Math|Conversions|ToTransform(Vector) _returnvalue_2))
  (bind (_outhit _returnvalue_4) (Collision|LineTraceByChannel _returnvalue_2 (+ _returnvalue_2 (* (Transformation|GetActorUpVector _returnvalue) -2e+02)) "TraceTypeQuery1" false 0 "None"))
  (if _returnvalue_4
    (switch Utilities|FlowControl|Switch|SwitchonEPhysicalSurface (Collision|GetSurfaceType _outhit)
      (:SurfaceType_Default
        (Class|FMODBlueprintStatics|PlayEventatLocation "/Game/FMOD/Events/Environment/Player/IdleCloth/Player_Idle_3.Player_Idle_3" _returnvalue_3 :!label _label))
      (:SurfaceType1
        (goto _label))
      (:SurfaceType2
        (goto _label))
      (:SurfaceType3
        (goto _label))
      (:SurfaceType4
        (goto _label))
      (:SurfaceType5
        (Class|FMODBlueprintStatics|PlayEventatLocation "/Game/FMOD/Events/Environment/Player/IdleCloth/DropInWater.DropInWater" _returnvalue_3)))
    (return)))