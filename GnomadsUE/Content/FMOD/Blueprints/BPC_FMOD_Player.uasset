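; Player audio component that drives FMOD music, ambience and object sounds.
; Starts forest, rough ambience and cave events on BeginPlay and stops them on EndPlay.
; Cat-trigger timer and grass-hiding events feed global FMOD parameters for danger riser, player noise and hidden state.
; Pick-up and drop play 2D events; drop also traces downward to play a positional sound by surface type, with a distinct water splash.
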(event Custom|DropObject
  ;[1 1 1] Pick up objects
  (Class|FMODBlueprintStatics|PlayEvent2D "/Game/FMOD/Events/Environment/Player/IdleCloth/Player_Idle_3.Player_Idle_3")
  (CallFunction|DropObjectonSurface))

(event Custom|HiddenInGrass
  (params (State :type Boolean))
  ;[1 1 1] Hidden in Grass
  (if State
    (Class|FMODBlueprintStatics|SetGlobalParameterbyName "HiddenInGrass" 1.0)
    (else
      (Class|FMODBlueprintStatics|SetGlobalParameterbyName "HiddenInGrass" 0.0))))

(event Custom|PickUpObject
  ;[1 1 1] Pick up objects
  (Class|FMODBlueprintStatics|PlayEvent2D "/Game/FMOD/Events/Environment/Player/IdleCloth/Player_Idle_4.Player_Idle_4"))

(event Custom|CatTriggeredMusic
  (params (CatTriggeredTimer :type Float%20%28double-precision%29))
  ;[1 1 1] Music
  (bind _output_get (Variables|Cat|SetCatTriggeredTimer CatTriggeredTimer))
  (if (> _output_get 0.99)
    (Class|FMODBlueprintStatics|SetGlobalParameterbyName "PlayerNoise" 1.0)
    (else
      (Class|FMODBlueprintStatics|SetGlobalParameterbyName "RiserDanger" (Variables|Cat|GetCatTriggeredTimer))
      (if (< (Variables|Cat|GetCatTriggeredTimer) 0.01)
        (Class|FMODBlueprintStatics|SetGlobalParameterbyName "PlayerNoise" 0.0)))))

(event EventEndPlay
  (params (EndPlayReason :type EEndPlayReason%20Enum :default "Destroyed"))
  ;[0.2031 0.2031 0.2031] Start/Stop Music system
  (Class|FMODBlueprintStatics|EventInstanceStop (stale EventBeginPlay _returnvalue) false)
  (Class|FMODBlueprintStatics|EventInstanceStop (stale EventBeginPlay _returnvalue_2) false)
  (Class|FMODBlueprintStatics|EventInstanceStop (stale EventBeginPlay _returnvalue_3) false))

(event EventBeginPlay
  ;[0.2031 0.2031 0.2031] Start/Stop Music system
  ;[0.375 0.375 0.375] Input danger between 0 - 1
  (Class|FMODBlueprintStatics|SetGlobalParameterbyName "Environment" (Variables|Default|GetNoiseLevel))
  (Class|FMODBlueprintStatics|SetGlobalParameterbyName "Environment" (Variables|Default|GetEnvironmentType))
  (bind _returnvalue (Class|FMODBlueprintStatics|PlayEvent2D "/Game/FMOD/Events/Music/Forest.Forest"))
  (bind _returnvalue_2 (Class|FMODBlueprintStatics|PlayEvent2D "/Game/FMOD/Events/Environment/Rough_ambience.Rough_ambience"))
  (bind _returnvalue_3 (Class|FMODBlueprintStatics|PlayEvent2D "/Game/FMOD/Events/Music/Cave.Cave")))

(fn DropObjectonSurface
  (bind _returnvalue (Components|GetOwner))
  (bind _returnvalue_2 (Transformation|GetActorLocation _returnvalue))
  (bind _returnvalue_3 (Math|Conversions|ToTransform(Vector) _returnvalue_2))
  (bind (_outhit _returnvalue_4) (Collision|LineTraceByChannel _returnvalue_2 (+ _returnvalue_2 (* (Transformation|GetActorUpVector _returnvalue) -2e+02)) "TraceTypeQuery1" false 0 "None"))
  (if _returnvalue_4
    (switch Utilities|FlowControl|Switch|SwitchonEPhysicalSurface (Collision|GetSurfaceType _outhit)
      (:SurfaceType_Default
        (Class|FMODBlueprintStatics|PlayEventatLocation "/Game/FMOD/Events/Environment/Player/IdleCloth/Player_Idle_3.Player_Idle_3" _returnvalue_3 :!label _label))
      (:SurfaceType1
        (goto _label))
      (:SurfaceType2
        (goto _label))
      (:SurfaceType3
        (goto _label))
      (:SurfaceType4
        (goto _label))
      (:SurfaceType5
        (Class|FMODBlueprintStatics|PlayEventatLocation "/Game/FMOD/Events/Environment/Player/IdleCloth/DropInWater.DropInWater" _returnvalue_3)))
    (return)))