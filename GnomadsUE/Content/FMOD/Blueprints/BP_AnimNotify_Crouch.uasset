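; An animation notify that plays the player's crouch footstep sound through FMOD, varied by the ground surface underfoot.
; On notify, it line-traces down from the owning actor and maps the hit physical surface (grass, stone, dirt, forest or water) to a numeric value.
; It plays the crouch footstep event in 2D and sets that value as the SurfaceType parameter.
; An at-location playback node remains but is never executed.
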(fn ReceivedNotify
  (params (MeshComp :type Skeletal%20Mesh%20Component%20Object%20Reference) (Animation :type Anim%20Sequence%20Base%20Object%20Reference) (EventReference :type Anim%20Notify%20Event%20Reference%20Structure%20%28by%20ref%29))
  (bind _returnvalue (Components|GetOwner MeshComp))
  (bind _returnvalue_2 (Transformation|GetActorLocation _returnvalue))
  (bind (_outhit _returnvalue_3) (Collision|LineTraceByChannel _returnvalue_2 (+ _returnvalue_2 (* (Transformation|GetActorUpVector _returnvalue) -2e+02)) "TraceTypeQuery1" false 0 "None"))
  (if _returnvalue_3
    (Utilities|FlowControl|Sequence
      (:then_0
        (switch Utilities|FlowControl|Switch|SwitchonEPhysicalSurface (Collision|GetSurfaceType _outhit)
          (:SurfaceType1
            (LocalVariables|SetSurface%20Type 0.5))
          (:SurfaceType2
            (LocalVariables|SetSurface%20Type 1.5))
          (:SurfaceType3
            (LocalVariables|SetSurface%20Type 2.5))
          (:SurfaceType4
            (LocalVariables|SetSurface%20Type 3.5))
          (:SurfaceType5
            (LocalVariables|SetSurface%20Type 4.5))))
      (:then_1
        (bind _returnvalue_4 (Class|FMODBlueprintStatics|PlayEvent2D "/Game/FMOD/Events/Environment/Player/Player_Footsteps_Crouch.Player_Footsteps_Crouch"))
        (Class|FMODBlueprintStatics|EventInstanceSetParameter _returnvalue_4 "SurfaceType" (LocalVariables|GetSurface%20Type))
        (return false)))
    (else
      (return false))))