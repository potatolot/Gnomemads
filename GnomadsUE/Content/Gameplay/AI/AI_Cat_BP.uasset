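; AI cat that, once activated, runs its behavior tree with the player and an initial roam location in the blackboard.
; While in its default state, a per-tick counter periodically re-randomizes the Director index that selects the roam area returned by GetAreaLocation.
; Overlaps on component R switch the AI state for catnip-tagged smell objects (ready ones or dropped items) and track nearby destructibles.
; Reset restores the default state.
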(event OnComponentBeginOverlap(r)
  (params (OverlappedComponent :type Primitive%20Component%20Object%20Reference) (OtherActor :type Actor%20Object%20Reference) (OtherComp :type Primitive%20Component%20Object%20Reference) (OtherBodyIndex :type Integer) (bFromSweep :type Boolean) (SweepResult :type Hit%20Result%20Structure%20%28by%20ref%29))
  (bind _aicontroller (Variables|Default|GetAIController))
  (bind _returnvalue (AI|GetBlackboard _aicontroller))
  ;[1 1 1] Smell Particle CallBack
  (if (Actor|ActorHasTag OtherActor "Catnip")
    (bind _assmelly_object_mat (Utilities|Casting|CastToSmellyObject_Mat OtherActor)
      (:then
        (bind _output_get (Variables|Default|SetSmellyObject _assmelly_object_mat))
        (if (Variables|/Game/Gameplay/SmellyObject_Mat.SmellyObject_Mat_C|GetReady _output_get)
          (AI|Components|Blackboard|SetValueasEnum _returnvalue (Utilities|Name|MakeLiteralName "AIState") (Utilities|Enum|LiteralenumAIState_Enum "NewEnumerator4") :!label _label)
          (AI|Components|Blackboard|SetValueasObject _returnvalue (Utilities|Name|MakeLiteralName "SmellObject") OtherActor)))
      (:CastFailed
        (bind _asdropped_object_bp (Utilities|Casting|CastToDroppedObject_BP OtherActor))
        (Variables|Default|SetDroppedSmell _asdropped_object_bp)
        (goto _label)))
    (else
      (bind _asdestructable_bp (Utilities|Casting|CastToDestructable_BP OtherActor))
      (Variables|Default|SetDestructable _asdestructable_bp))))

(event OnComponentEndOverlap(r)
  (params (OverlappedComponent :type Primitive%20Component%20Object%20Reference) (OtherActor :type Actor%20Object%20Reference) (OtherComp :type Primitive%20Component%20Object%20Reference) (OtherBodyIndex :type Integer))
  ;[1 1 1] Smell Particle CallBack
  (Utilities|Casting|CastToDestructable_BP OtherActor
    (:then
      (Variables|Default|SetDestructable 0))
    (:CastFailed
      (Utilities|Casting|CastToDroppedObject_BP OtherActor)
      (Variables|Default|SetDroppedSmell 0))))

(event Custom|Activcate
  (Variables|Default|SetActive true)
  ;[1 1 1] Get reference to AI controller
  (bind _asai_cat_controller (Utilities|Casting|CastToAI_Cat_Controller (Pawn|GetController)))
  (bind _output_get (Variables|Default|SetAIController _asai_cat_controller))
  ;[1 1 1] Activate Behaviour Tree
  (AI|RunBehaviorTree _output_get "/Game/Gameplay/AI/AI_Cat_BT.AI_Cat_BT")
  (bind _asbp_third_person_character_stealth (Utilities|Casting|CastToBP_ThirdPersonCharacter_Stealth (Game|GetPlayerCharacter 0)))
  (AI|Components|Blackboard|SetValueasObject (AI|GetBlackboard (Variables|Default|GetAIController)) (Utilities|Name|MakeLiteralName "PlayerObject") _asbp_third_person_character_stealth)
  (bind _location (CallFunction|GetAreaLocation))
  (AI|Components|Blackboard|SetValueasVector (AI|GetBlackboard (Variables|Default|GetAIController)) (Utilities|Name|MakeLiteralName "RoamLocation") _location))

(event Custom|Reset
  (AI|Components|Blackboard|SetValueasEnum (AI|GetBlackboard (Variables|Default|GetAIController)) (Utilities|Name|MakeLiteralName "AIState") (Utilities|Enum|LiteralenumAIState_Enum "NewEnumerator0")))

(event EventTick
  (params (DeltaSeconds :type Float%20%28single-precision%29))
  (bind _areas (Variables|Default|GetAreas))
  (bind _returnvalue (Utilities|Array|Length _areas))
  (bind _returnvalue_2 (- _returnvalue 1))
  (bind _returnvalue_3 (Math|Random|RandomInteger _returnvalue_2))
  (if (Variables|Default|GetActive)
    (if (== (Class|BlackboardComponent|GetValueasEnum (AI|GetBlackboard (Variables|Default|GetAIController)) (Utilities|Name|MakeLiteralName "AIState")) 0)
      (bind _result (Math|Float|IncrementFloat (Variables|Default|GetDirectorChanger))
        (:%20%20
          (if (> _result 5e+02)
            (Variables|Default|SetDirectorChanger 0.0)
            (if (== _returnvalue_3 (Variables|Default|GetDirector))
              (Variables|Default|SetDirector 0)
              (elif (== _returnvalue_3 _returnvalue_2)
                (bind _result_2 (Math|Integer|DecrementInt _returnvalue_3)
                  (:%20%20
                    (Variables|Default|SetDirector _result_2)))
                (else
                  (bind _result_3 (Math|Integer|IncrementInt _returnvalue_3)
                    (:%20%20
                      (Variables|Default|SetDirector _result_3))))))))))))

(fn ConstructionScript)

(fn GetAreaLocation
  (return (Transformation|GetActorLocation (Utilities|Array|Get(acopy) (Variables|Default|GetAreas) (Variables|Default|GetDirector)))))