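; FallingTree_BP is a one-shot trigger for a scripted falling-tree moment in a stealth level.
; When the stealth character enters the box, it teleports the Cat to a spawn point, sets its Director value, and plays the tree Level Sequence with a sound event.
; It also auto-moves the player to a goal and hides the GrassDirection component for a short delay.
; Older input-mode, checkpoint and AI-state logic remains disconnected.
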(event OnComponentBeginOverlap(Box)
  (params (OverlappedComponent :type Primitive%20Component%20Object%20Reference) (OtherActor :type Actor%20Object%20Reference) (OtherComp :type Primitive%20Component%20Object%20Reference) (OtherBodyIndex :type Integer) (bFromSweep :type Boolean) (SweepResult :type Hit%20Result%20Structure%20%28by%20ref%29))
  (bind _asbp_third_person_character_stealth (Utilities|Casting|CastToBP_ThirdPersonCharacter_Stealth OtherActor))
  (if (not (Variables|Default|GetTriggered))
    (Variables|Default|SetTriggered true)
    (Transformation|SetActorLocation (Variables|Default|GetCat) (Transformation|GetActorLocation (Variables|Default|GetCatSpawn)) false false)
    (Rendering|SetVisibility (Variables|/Game/ThirdPerson/Blueprints/Stealth_Character/BP_ThirdPersonCharacter_Stealth.BP_ThirdPersonCharacter_Stealth_C|GetGrassDirection _asbp_third_person_character_stealth) false true)
    (bind _outactor (Sequencer|Player|CreateLevelSequencePlayer "/Game/Gameplay/Animatics/Tree_Sequence.Tree_Sequence" (Utilities|Struct|MakeMovieSceneSequencePlaybackSettings false "(Value=0)" 1.0 0.0 false false false false false false false true)))
    (Sequencer|Player|Play (Variables|/Script/LevelSequence.LevelSequenceActor|GetSequencePlayer _outactor) :!class /Script/MovieScene.MovieSceneSequencePlayer)
    (Default|ChangeCrouch _asbp_third_person_character_stealth false)
    (AI|Navigation|SimpleMovetoLocation (Game|GetPlayerController 0) (Transformation|GetActorLocation (Variables|Default|GetGoal)))
    (Class|FMODBlueprintStatics|PlayEvent2D "/Game/FMOD/Events/Environment/Flora/FallingTree.FallingTree")
    (Variables|/Game/Gameplay/AI/AI_Cat_BP.AI_Cat_BP_C|SetDirector (Variables|Default|GetCat) 2)
    (Utilities|FlowControl|Delay 2.0)
    (Rendering|SetVisibility (Variables|/Game/ThirdPerson/Blueprints/Stealth_Character/BP_ThirdPersonCharacter_Stealth.BP_ThirdPersonCharacter_Stealth_C|GetGrassDirection _asbp_third_person_character_stealth) true true)))

(fn ConstructionScript)