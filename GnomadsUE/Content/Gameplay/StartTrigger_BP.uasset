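; One-shot box trigger that plays a camera level sequence on the first overlap and stages the stealth player character for it.
; If the overlapping actor is that character, it activates the cat actor, hides the character's Nope component, stops and crouches it, auto-moves it to the trigger and locks input to UI only.
; A timer matched to the sequence duration shows Nope again and restores game input.
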(event OnComponentBeginOverlap(Box)
  (params (OverlappedComponent :type Primitive%20Component%20Object%20Reference) (OtherActor :type Actor%20Object%20Reference) (OtherComp :type Primitive%20Component%20Object%20Reference) (OtherBodyIndex :type Integer) (bFromSweep :type Boolean) (SweepResult :type Hit%20Result%20Structure%20%28by%20ref%29))
  ;[1 1 1] Camera Animation
  (if (not (Variables|Default|GetTriggered))
    (Variables|Default|SetTriggered true)
    (bind _outactor (Sequencer|Player|CreateLevelSequencePlayer (Variables|Default|GetSequence)))
    (Sequencer|Player|Play (Variables|/Script/LevelSequence.LevelSequenceActor|GetSequencePlayer _outactor) :!class /Script/MovieScene.MovieSceneSequencePlayer)
    (Utilities|Time|SetTimerbyEvent (delegate Custom|Reset) (Class|TimeManagementBlueprintLibrary|ToSeconds(QualifiedFrameTime) (Media|MediaPlayer|GetDuration (Variables|/Script/LevelSequence.LevelSequenceActor|GetSequencePlayer _outactor))))
    (bind _asbp_third_person_character_stealth (Utilities|Casting|CastToBP_ThirdPersonCharacter_Stealth OtherActor))
    (Default|Activcate (Variables|Default|GetCatActor))
    (Rendering|SetVisibility (Variables|/Game/ThirdPerson/Blueprints/Stealth_Character/BP_ThirdPersonCharacter_Stealth.BP_ThirdPersonCharacter_Stealth_C|GetNope _asbp_third_person_character_stealth) false false)
    (Variables|/Script/Engine.MovementComponent|SetVelocity (Variables|/Script/Engine.Character|GetCharacterMovement _asbp_third_person_character_stealth) "0, 0, 0")
    (Default|ChangeCrouch _asbp_third_person_character_stealth true)
    (AI|Navigation|SimpleMovetoLocation (Game|GetPlayerController 0) (Transformation|GetActorLocation))
    (Input|SetInputModeUIOnly (Game|GetPlayerController 0) 0 "LockAlways" true)))

(event Custom|Reset
  (bind _asbp_third_person_character_stealth (Utilities|Casting|CastToBP_ThirdPersonCharacter_Stealth (Game|GetPlayerCharacter 0)))
  (Rendering|SetVisibility (Variables|/Game/ThirdPerson/Blueprints/Stealth_Character/BP_ThirdPersonCharacter_Stealth.BP_ThirdPersonCharacter_Stealth_C|GetNope _asbp_third_person_character_stealth) true false)
  (Input|SetInputModeGameOnly (Game|GetPlayerController 0) false))

(fn ConstructionScript)