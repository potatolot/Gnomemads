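; Cave trigger volume that changes post-process exposure when the stealth third-person character enters or leaves a cave.
; On overlap begin, the ChangeExposure timeline drives exposure compensation on a post-process volume.
; On overlap end, exposure compensation snaps back to a fixed value without fading.
; An IsInCave flag guards both transitions, and debug strings print on each.
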(event OnComponentBeginOverlap(CollisionComponent)
  (params (OverlappedComponent :type Primitive%20Component%20Object%20Reference) (OtherActor :type Actor%20Object%20Reference) (OtherComp :type Primitive%20Component%20Object%20Reference) (OtherBodyIndex :type Integer) (bFromSweep :type Boolean) (SweepResult :type Hit%20Result%20Structure%20%28by%20ref%29))
  ;[1 1 1] Cave Exposure
  (Utilities|Casting|CastToBP_ThirdPersonCharacter_Stealth OtherActor)
  (if (not (Variables|Default|GetIs%20in%20Cave?))
    (Actor|GetActorOfClass "/Script/Engine.PostProcessVolume")
    (Development|PrintString "hello")
    (Variables|Default|SetIs%20In%20Cave? true)
    (bind _exposurevalue (Timeline|ChangeExposure PlayFromStart)
      (:Update
        (Utilities|Struct|SetmembersinPostProcessSettings (Variables|/Script/Engine.PostProcessVolume|GetSettings (Variables|Default|GetPost%20Processing%20Volume)) _exposurevalue)))))

(event OnComponentEndOverlap(CollisionComponent)
  (params (OverlappedComponent :type Primitive%20Component%20Object%20Reference) (OtherActor :type Actor%20Object%20Reference) (OtherComp :type Primitive%20Component%20Object%20Reference) (OtherBodyIndex :type Integer))
  ;[1 1 1] Cave Exposure
  (Utilities|Casting|CastToBP_ThirdPersonCharacter_Stealth OtherActor)
  (if (Variables|Default|GetIs%20in%20Cave?)
    (Actor|GetActorOfClass "/Script/Engine.PostProcessVolume")
    (Development|PrintString "goodbye")
    (Utilities|Struct|SetmembersinPostProcessSettings (Variables|/Script/Engine.PostProcessVolume|GetSettings (Variables|Default|GetPost%20Processing%20Volume)) 1.0)
    (Variables|Default|SetIs%20In%20Cave? false)))

(event EventBeginPlay)

(event Collision|EventActorBeginOverlap
  (params (OtherActor :type Actor%20Object%20Reference)))

(event EventTick
  (params (DeltaSeconds :type Float%20%28single-precision%29)))

(fn ConstructionScript)