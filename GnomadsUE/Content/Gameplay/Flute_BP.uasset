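; Flute component for the stealth third-person character that plays a whistle on the Flute_MI input to make noise AI hearing can detect.
; Outside Tutorial mode, it reports a noise event at the owner's location and calls Whistle on the character's FMOD player.
; Every press also shows FluteVFX for a short delay.
; The character reference is cached after the sound step, so the first press's whistle relies on it already being set.
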(event Input|EnhancedActionEvents|EnhancedInputActionFlute_MI
  (params (ActionValue :type Boolean) (ElapsedSeconds :type Float%20%28double-precision%29) (TriggeredSeconds :type Float%20%28double-precision%29) (InputAction :type Input%20Action%20Object%20Reference :default "/Game/Gameplay/Input/Actions/Flute_MI.Flute_MI"))
  (bind _self self)
  (bind _returnvalue (Components|GetOwner _self))
  (Utilities|FlowControl|Sequence
    (:then_0
      (if (not (Variables|Default|GetTutorial))
        (Class|AISenseHearing|ReportNoiseEvent (Transformation|GetActorLocation _returnvalue) 1.0 _returnvalue 2e+03 "None")
        (bind _bpc_fmod_player (Variables|/Game/Characters/KabouterPlayer/BP_ThirdPersonCharacter_Stealth.BP_ThirdPersonCharacter_Stealth_C|GetBPC_FMOD_Player (stale _asbp_third_person_character_stealth))
          (:then
            (Default|Whistle _bpc_fmod_player true))
          (:else))))
    (:then_1
      (bind _asbp_third_person_character_stealth (Utilities|Casting|CastToBP_ThirdPersonCharacter_Stealth (Components|GetOwner)))
      (Rendering|SetVisibility (Variables|/Game/Characters/KabouterPlayer/BP_ThirdPersonCharacter_Stealth.BP_ThirdPersonCharacter_Stealth_C|GetfluteVFX _asbp_third_person_character_stealth) true true)
      (Utilities|FlowControl|Delay 2.0)
      (Rendering|SetVisibility (Variables|/Game/Characters/KabouterPlayer/BP_ThirdPersonCharacter_Stealth.BP_ThirdPersonCharacter_Stealth_C|GetfluteVFX _asbp_third_person_character_stealth) false true))))

(event EventBeginPlay)

(event EventTick
  (params (DeltaSeconds :type Float%20%28single-precision%29)))