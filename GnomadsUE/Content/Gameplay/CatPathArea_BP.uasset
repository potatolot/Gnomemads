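; CatPathArea_BP is a trigger area that switches the cat AI's patrol path as the stealth player progresses through checkpoints.
; It caches the single CatAI_BluePrint on BeginPlay.
; When the player overlaps the Box with CurrentCheckPoint equal to PlayerCP, it assigns its Path to the cat and resets the path index.
; If SetCheckpoint is set, it also updates the player's checkpoint once and prints it for debugging.
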(event OnComponentBeginOverlap(Box)
  (params (OverlappedComponent :type Primitive%20Component%20Object%20Reference) (OtherActor :type Actor%20Object%20Reference) (OtherComp :type Primitive%20Component%20Object%20Reference) (OtherBodyIndex :type Integer) (bFromSweep :type Boolean) (SweepResult :type Hit%20Result%20Structure%20%28by%20ref%29))
  (bind _cat (Variables|Default|GetCat))
  (bind _asbp_third_person_character_stealth (Utilities|Casting|CastToBP_ThirdPersonCharacter_Stealth OtherActor))
  (if (== (Variables|Default|GetPlayerCP) (Variables|/Game/ThirdPerson/Blueprints/Stealth_Character/BP_ThirdPersonCharacter_Stealth.BP_ThirdPersonCharacter_Stealth_C|GetCurrentCheckPoint _asbp_third_person_character_stealth))
    (Variables|/Game/Characters/Cat/CatAI_BluePrint.CatAI_BluePrint_C|SetCurrentPath _cat (Variables|Default|GetPath))
    (Variables|/Game/Characters/Cat/CatAI_BluePrint.CatAI_BluePrint_C|SetPathIndex _cat 0)
    (if (Variables|Default|GetSetCheckpoint)
      (bind _output_get (Variables|/Game/ThirdPerson/Blueprints/Stealth_Character/BP_ThirdPersonCharacter_Stealth.BP_ThirdPersonCharacter_Stealth_C|SetCurrentCheckPoint _asbp_third_person_character_stealth (Variables|Default|GetCheckPoint)))
      (Variables|Default|SetSetCheckpoint false)
      (Development|PrintString (Utilities|String|ToString(Integer) _output_get)))))

(event EventBeginPlay
  (bind _returnvalue (Actor|GetActorOfClass "/Game/Characters/Cat/CatAI_BluePrint.CatAI_BluePrint_C"))
  (Variables|Default|SetCat _returnvalue))

(event Collision|EventActorBeginOverlap
  (params (OtherActor :type Actor%20Object%20Reference)))

(event EventTick
  (params (DeltaSeconds :type Float%20%28single-precision%29)))

(fn ConstructionScript)