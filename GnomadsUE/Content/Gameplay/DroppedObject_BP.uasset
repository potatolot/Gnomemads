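; Dropped-object pickup actor that the stealth third-person character can collect to carry.
; Box overlap shows a text prompt and binds Pickup to the character's PickUp dispatcher; leaving hides the prompt without unbinding.
; Pickup flags the character as holding, reveals its carried-object component, sets a fixed walk speed and destroys this actor.
; A separate DestroyDropped event removes the actor without granting the pickup.
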(event OnComponentBeginOverlap(Box)
  (params (OverlappedComponent :type Primitive%20Component%20Object%20Reference) (OtherActor :type Actor%20Object%20Reference) (OtherComp :type Primitive%20Component%20Object%20Reference) (OtherBodyIndex :type Integer) (bFromSweep :type Boolean) (SweepResult :type Hit%20Result%20Structure%20%28by%20ref%29))
  (bind _asbp_third_person_character_stealth (Utilities|Casting|CastToBP_ThirdPersonCharacter_Stealth OtherActor))
  (Rendering|SetVisibility (Variables|Default|GetTextRender) true false)
  (EventDispatchers|BindEventtoPickUp _asbp_third_person_character_stealth (delegate Custom|Pickup)))

(event OnComponentEndOverlap(Box)
  (params (OverlappedComponent :type Primitive%20Component%20Object%20Reference) (OtherActor :type Actor%20Object%20Reference) (OtherComp :type Primitive%20Component%20Object%20Reference) (OtherBodyIndex :type Integer))
  (Utilities|Casting|CastToBP_ThirdPersonCharacter_Stealth OtherActor)
  (Rendering|SetVisibility (Variables|Default|GetTextRender) false false))

(event Custom|Pickup
  (Variables|/Game/ThirdPerson/Blueprints/Stealth_Character/BP_ThirdPersonCharacter_Stealth.BP_ThirdPersonCharacter_Stealth_C|SetHoldinObject (stale OnComponentBeginOverlap(Box) _asbp_third_person_character_stealth) true)
  (Rendering|SetVisibility (Variables|/Game/ThirdPerson/Blueprints/Stealth_Character/BP_ThirdPersonCharacter_Stealth.BP_ThirdPersonCharacter_Stealth_C|GetPickedUpObject (stale OnComponentBeginOverlap(Box) _asbp_third_person_character_stealth)) true false)
  (Variables|/Script/Engine.CharacterMovementComponent|SetMaxWalkSpeed (Variables|/Script/Engine.Character|GetCharacterMovement (stale OnComponentBeginOverlap(Box) _asbp_third_person_character_stealth)) 1.5e+02)
  (Actor|DestroyActor))

(event Custom|DestroyDropped
  (Actor|DestroyActor))

(event EventBeginPlay)

(event Collision|EventActorBeginOverlap
  (params (OtherActor :type Actor%20Object%20Reference)))

(event EventTick
  (params (DeltaSeconds :type Float%20%28single-precision%29)))

(fn ConstructionScript)